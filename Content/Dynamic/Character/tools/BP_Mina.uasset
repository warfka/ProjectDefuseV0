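; BP_Mina is a physics-simulated mine that explodes 1.5 seconds after something overlaps its Check trigger.
; Detonation plays sound and Niagara, hides the mesh, briefly expands the Damage sphere, then later destroys the actor.
; That sphere's overlap runs a multi-sphere trace and applies heavy damage to blocking hits.
; AnyDamage repeats the detonation, but only if Dead is already set and HP stays above zero, apparently inverted checks.
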(event OnComponentBeginOverlap(Check)
  (params (OverlappedComponent :type Primitive%20Component%20Object%20Reference) (OtherActor :type Actor%20Object%20Reference) (OtherComp :type Primitive%20Component%20Object%20Reference) (OtherBodyIndex :type Integer) (bFromSweep :type Boolean) (SweepResult :type Hit%20Result%20Structure%20%28by%20ref%29))
  (bind _damage (Variables|Default|GetDamage))
  (if (not (Variables|Default|GetDead))
    (Audio|PlaySoundatLocation "/Game/Static/FPWeapon/Audio/FirstPersonTemplateWeaponFire02.FirstPersonTemplateWeaponFire02" (Transformation|GetActorLocation) "0, 0, 0" 1.0 1.0 0.0 0 0 0 0)
    (Utilities|FlowControl|Delay 1.5)
    (Variables|Default|SetDead true)
    (Audio|PlaySoundatLocation "/Game/Dynamic/StarterContent/Audio/Explosion01.Explosion01" (Transformation|GetActorLocation) "0, 0, 0" 1.0 1.0 0.0 0 0 0 0)
    (Collision|SetCollisionEnabled (Variables|Default|GetCheck) "NoCollision")
    (Components|Activation|SetActive (Variables|Default|GetNiagara) true false)
    (Rendering|SetVisibility (Variables|Default|GetMina) false false)
    (Utilities|IsValid _damage
      (:Is%20Valid
        (Collision|SetCollisionEnabled _damage "QueryAndPhysics")
        (Components|Sphere|SetSphereRadius _damage 2e+02 true)
        (Utilities|FlowControl|Delay 0.2)
        (Components|DestroyComponent _damage)
        (Utilities|FlowControl|Delay 6.0)
        (Actor|DestroyActor)))))

(event OnComponentBeginOverlap(Damage)
  (params (OverlappedComponent :type Primitive%20Component%20Object%20Reference) (OtherActor :type Actor%20Object%20Reference) (OtherComp :type Primitive%20Component%20Object%20Reference) (OtherBodyIndex :type Integer) (bFromSweep :type Boolean) (SweepResult :type Hit%20Result%20Structure%20%28by%20ref%29))
  (bind _damage (Variables|Default|GetDamage))
  (bind _returnvalue (Transformation|GetWorldLocation _damage))
  (bind _outhits (Collision|MultiSphereTraceForObjects _returnvalue (+ _returnvalue (* (Math|Vector|GetForwardVector _damage) "200.000000,0.000000,0.000000")) 2e+02 (Utilities|Array|MakeArray "ObjectTypeQuery8" "ObjectTypeQuery9") false 0 "None"))
  (for _array_element _outhits
    (if (.bBlockingHit (Collision|BreakHitResult _array_element))
      (Game|Damage|ApplyDamage 0 5e+02 0 self))))

(event EventBeginPlay
  (Physics|SetSimulatePhysics (Variables|Default|GetBox) true)
  (Collision|SetCollisionEnabled (Variables|Default|GetDamage) "QueryOnly"))

(event Game|Damage|EventAnyDamage
  (params (Damage :type Float%20%28single-precision%29) (DamageType :type Damage%20Type%20Object%20Reference) (InstigatedBy :type Controller%20Object%20Reference) (DamageCauser :type Actor%20Object%20Reference))
  (if (Variables|Default|GetDead)
    (Variables|Default|SetHP (- (Variables|Default|GetHP) Damage))
    (Utilities|FlowControl|Sequence
      (:then_0
        (Audio|PlaySoundatLocation "/Game/Dynamic/StarterContent/Audio/Explosion01.Explosion01" (Transformation|GetActorLocation) "0, 0, 0" 1.0 1.0 0.0 0 0 0 0))
      (:then_1
        (if (not (<= (Variables|Default|GetHP) 0.0))
          (Variables|Default|SetDead true)
          (Utilities|FlowControl|Delay 1.0)
          (Audio|PlaySoundatLocation "/Game/Dynamic/StarterContent/Audio/Explosion01.Explosion01" (Transformation|GetActorLocation) "0, 0, 0" 1.0 1.0 0.0 0 0 0 0)
          (Collision|SetCollisionEnabled (Variables|Default|GetCheck) "NoCollision")
          (Components|Activation|SetActive (Variables|Default|GetNiagara) true false)
          (Rendering|SetVisibility (Variables|Default|GetMina) false false)
          (Utilities|IsValid (Variables|Default|GetDamage)
            (:Is%20Valid
              (Collision|SetCollisionEnabled (Variables|Default|GetDamage) "QueryAndPhysics")
              (Components|Sphere|SetSphereRadius (Variables|Default|GetDamage) 2e+02 true)
              (Utilities|FlowControl|Delay 0.2)
              (Components|DestroyComponent (Variables|Default|GetDamage))
              (Utilities|FlowControl|Delay 6.0)
              (Actor|DestroyActor))))))))

(fn ConstructionScript)